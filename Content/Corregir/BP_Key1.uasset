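; BP_Key1 is a collectible key for the puzzle door minigame.
; When the third-person character overlaps its Capsule, it increments ItemsCollected on the BP_PuzzleDoor found by class lookup, then hides its Cylinder and disables collision.
; Tick polls that door's ReiniciarMinijuego flag every frame and, while it is true, restores visibility and collision so the key can be collected again.
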(event `self.ReceiveTick`
  (params (DeltaSeconds :type "Float (single-precision)"))
  (bind _returnvalue (`GameplayStatics.GetActorOfClass` "/Game/Corregir/Mapa/BP_PuzzleDoor.BP_PuzzleDoor_C"))
  (if (`/Game/Corregir/Mapa/BP_PuzzleDoor.ReiniciarMinijuego` _returnvalue)
    (`SceneComponent.SetVisibility` (`self.Cylinder`) true false)
    (`PrimitiveComponent.SetCollisionEnabled` (`self.Capsule`) "QueryAndPhysics")))

(event `self.Capsule.OnComponentBeginOverlap`
  (params (OverlappedComponent :type "PrimitiveComponent Object Reference") (OtherActor :type "Actor Object Reference") (OtherComp :type "PrimitiveComponent Object Reference") (OtherBodyIndex :type Integer) (bFromSweep :type Boolean) (SweepResult :type "HitResult Structure (by ref)"))
  (cast `/Game/Corregir/BP_ThirdPersonCharacter` OtherActor)
  (bind _returnvalue (`GameplayStatics.GetActorOfClass` "/Game/Corregir/Mapa/BP_PuzzleDoor.BP_PuzzleDoor_C"))
  (set `/Game/Corregir/Mapa/BP_PuzzleDoor.itemsCollected` (+ (`/Game/Corregir/Mapa/BP_PuzzleDoor.itemsCollected` _returnvalue) 1) _returnvalue)
  (`PrimitiveComponent.SetCollisionEnabled` (`self.Capsule`) "NoCollision")
  (`SceneComponent.SetVisibility` (`self.Cylinder`) false false))

(fn `UserConstructionScript`)